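; VR player pawn for the MG4 ship minigame, handling the start screen, pausing and hand-pointer UI clicks.
; BeginPlay freezes play with zero global time dilation, shows the start widget and both pointers' debug rays, and caches the starting transform.
; The X button likewise freezes time, shows the pause widget and rays, and pauses the movie player and BGM.
; Left and right triggers press and release left-mouse clicks through their WidgetInteraction components.
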(event Input|EnhancedActionEvents|EnhancedInputActionIA_TriggerL
  (params (ActionValue :type Boolean) (ElapsedSeconds :type Float%20%28double-precision%29) (TriggeredSeconds :type Float%20%28double-precision%29) (InputAction :type Input%20Action%20Object%20Reference :default "/Game/PlayerInput/GN/IA_TriggerL.IA_TriggerL"))
  (bind _widgetinteractionl (Variables|Default|GetWidgetInteractionL))
  (:Triggered
    (Class|WidgetInteractionComponent|PressPointerKey _widgetinteractionl "LeftMouseButton"))
  (:Completed
    (Class|WidgetInteractionComponent|ReleasePointerKey _widgetinteractionl "LeftMouseButton")))

(event Input|EnhancedActionEvents|EnhancedInputActionIA_TriggerR
  (params (ActionValue :type Boolean) (ElapsedSeconds :type Float%20%28double-precision%29) (TriggeredSeconds :type Float%20%28double-precision%29) (InputAction :type Input%20Action%20Object%20Reference :default "/Game/PlayerInput/GN/IA_TriggerR.IA_TriggerR"))
  (bind _widgetinteractionr (Variables|Default|GetWidgetInteractionR))
  (:Triggered
    (Class|WidgetInteractionComponent|PressPointerKey _widgetinteractionr "LeftMouseButton"))
  (:Completed
    (Class|WidgetInteractionComponent|ReleasePointerKey _widgetinteractionr "LeftMouseButton")))

(event Input|EnhancedActionEvents|EnhancedInputActionIA_btnX
  (params (ActionValue :type Boolean) (ElapsedSeconds :type Float%20%28double-precision%29) (TriggeredSeconds :type Float%20%28double-precision%29) (InputAction :type Input%20Action%20Object%20Reference :default "/Game/PlayerInput/GN/IA_btnX.IA_btnX"))
  (bind _bgm (Variables|Default|Getbgm))
  (:Triggered
    (Rendering|SetVisibility (Variables|Default|GetPauseWidget) true false)
    ;[1 1 1] 일시정지 기능
    (Utilities|Time|SetGlobalTimeDilation 0.0)
    (Variables|/Script/UMG.WidgetInteractionComponent|SetbShowDebug (Variables|Default|GetWidgetInteractionR) true)
    (Variables|/Script/UMG.WidgetInteractionComponent|SetbShowDebug (Variables|Default|GetWidgetInteractionL) true)
    (Class|MoviePlayerActor|PausedMovie (Variables|Default|GetmoviePlayer))
    (Utilities|IsValid _bgm
      (:Is%20Valid
        (Class|AudioComponent|SetPaused _bgm true)))))

(event EventBeginPlay
  (Utilities|Time|SetGlobalTimeDilation 0.0)
  (Variables|/Script/UMG.WidgetInteractionComponent|SetbShowDebug (Variables|Default|GetWidgetInteractionR) true)
  (Variables|/Script/UMG.WidgetInteractionComponent|SetbShowDebug (Variables|Default|GetWidgetInteractionL) true)
  (Rendering|SetVisibility (Variables|Default|GetStartWidget) true false)
  (Variables|Default|SetInit (Transformation|GetActorTransform)))

(fn ConstructionScript)