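; BP_MoviePlayer_MG4 is a movie player actor that shows a media source on its VideoPlayer component with sound.
; The construction script applies the media material, and BeginPlay links MediaSound to the MediaPlayer, binds the end-reached event and calls Play on the player.
; Its Play event opens the source when the Playing flag is false and otherwise resumes playback.
; Pause pauses the player, and reaching the end clears the flag.
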(event Custom|EndVideo
  (Variables|Default|SetPlaying false))

(event Custom|Pause
  (Sequencer|Player|Pause (Variables|Default|GetMediaPlayer)))

(event Custom|Play
  (bind _mediaplayer (Variables|Default|GetMediaPlayer))
  (if (Variables|Default|GetPlaying)
    (Media|MediaPlayer|Play _mediaplayer :!class /Script/MediaAssets.MediaPlayer)
    (else
      (Media|MediaPlayer|OpenSource _mediaplayer (Variables|Default|GetMediaSource))
      (Variables|Default|SetPlaying true))))

(event EventBeginPlay
  (bind _mediaplayer (Variables|Default|GetMediaPlayer))
  (Media|MediaSoundComponent|SetMediaPlayer (Variables|Default|GetMediaSound) (Variables|Default|GetMediaPlayer))
  (Variables|Default|SetPlaying false)
  (Media|MediaPlayer|BindEventtoOnEndReached _mediaplayer (delegate Custom|EndVideo))
  (Media|MediaPlayer|Play _mediaplayer :!class /Script/MediaAssets.MediaPlayer))

(fn ConstructionScript
  (Rendering|Material|SetMaterial (Variables|Default|GetVideoPlayer) 0 (Variables|Default|GetMediaMaterial)))