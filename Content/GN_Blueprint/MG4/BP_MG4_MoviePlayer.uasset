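; BP_MG4_MoviePlayer is an MG4 actor that plays an ending Level Sequence and then opens the Gallery level.
; On BeginPlay it caches the LevelSequenceActor found in the level.
; Tick polls CurrTime, which this graph never updates; at two seconds or more it sets and plays EndLevelSequence on every tick.
; A short Delay follows before the level change.
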(event EventBeginPlay
  (bind _returnvalue (Actor|GetActorOfClass "/Script/LevelSequence.LevelSequenceActor"))
  (Variables|Default|SetLevelSequence _returnvalue))

(event Collision|EventActorBeginOverlap
  (params (OtherActor :type Actor%20Object%20Reference)))

(event EventTick
  (params (DeltaSeconds :type Float%20%28single-precision%29))
  (bind _levelsequence (Variables|Default|GetLevelSequence))
  (if (>= (Variables|Default|GetcurrTime) 2.0)
    (Class|LevelSequenceActor|SetSequence _levelsequence "/Game/Sequence/EndLevelSequence.EndLevelSequence")
    (Sequencer|Player|Play (Variables|/Script/LevelSequence.LevelSequenceActor|GetSequencePlayer _levelsequence) :!class /Script/MovieScene.MovieSceneSequencePlayer)
    (Utilities|FlowControl|Delay 2.0)
    (Game|OpenLevel(byObjectReference) "/Game/Levels/Gallery.Gallery")))

(fn ConstructionScript)