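; BP_spawnPos1-2 is a trigger actor that shows a widget and reveals the player's widget pointers when a capsule component enters its box.
; On BeginPlay it waits briefly, then caches the BP_mainPlayer actor.
; The box overlap filters for any capsule component, makes Widget21 visible, and turns on ShowDebug for the cached player's left and right WidgetInteraction components.
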(event OnComponentBeginOverlap(Box)
  (params (OverlappedComponent :type Primitive%20Component%20Object%20Reference) (OtherActor :type Actor%20Object%20Reference) (OtherComp :type Primitive%20Component%20Object%20Reference) (OtherBodyIndex :type Integer) (bFromSweep :type Boolean) (SweepResult :type Hit%20Result%20Structure%20%28by%20ref%29))
  (Utilities|Casting|CastToCapsuleComponent OtherComp)
  (Rendering|SetVisibility (Variables|Default|GetWidget2-1) true false)
  (bind _output_get (Variables|Default|SetWidget%20Interaction%20L (Variables|/Game/GN_Blueprint/Main/BP_mainPlayer.BP_mainPlayer_C|GetWidgetInteractionL (stale EventBeginPlay _returnvalue))))
  (bind _output_get_2 (Variables|Default|SetWidget%20Interaction%20R (Variables|/Game/GN_Blueprint/Main/BP_mainPlayer.BP_mainPlayer_C|GetWidgetInteractionR (stale EventBeginPlay _returnvalue))))
  (Variables|/Script/UMG.WidgetInteractionComponent|SetbShowDebug _output_get true)
  (Variables|/Script/UMG.WidgetInteractionComponent|SetbShowDebug _output_get_2 true))

(event EventBeginPlay
  (Utilities|FlowControl|Delay 1.0)
  (bind _returnvalue (Actor|GetActorOfClass "/Game/GN_Blueprint/Main/BP_mainPlayer.BP_mainPlayer_C")))

(fn ConstructionScript)