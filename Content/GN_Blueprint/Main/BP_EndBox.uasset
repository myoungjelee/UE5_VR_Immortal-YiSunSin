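; BP_EndBox is a trigger box that shows an end-text UI when the player's head enters it and removes it on exit.
; On head overlap it spawns UI_txtEnd at a fixed spot, reveals its widget after a short delay and turns on both widget-interaction debug rays.
; It also writes a position and the controller rotation to YiSunSinInstance.
; Leaving stops any audio, destroys the UI and hides the rays.
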(event OnComponentBeginOverlap(Box)
  (params (OverlappedComponent :type Primitive%20Component%20Object%20Reference) (OtherActor :type Actor%20Object%20Reference) (OtherComp :type Primitive%20Component%20Object%20Reference) (OtherBodyIndex :type Integer) (bFromSweep :type Boolean) (SweepResult :type Hit%20Result%20Structure%20%28by%20ref%29))
  (bind _yi_sun_sin_instance (Variables|Default|GetYi%20Sun%20Sin%20Instance))
  (if (Utilities|String|Contains (Utilities|GetObjectName OtherComp) "Head")
    (bind _returnvalue (Game|SpawnActorfromClass "/Game/GN_UI/Main/Ending/UI_txtEnd.UI_txtEnd_C" (Math|Transform|MakeTransform "-570.000000,560.000000,250.000000" "0, 0, 0" "1.000000,1.000000,1.000000") "Undefined" 0 0))
    (bind _output_get (Variables|Default|SetWidgetActor _returnvalue))
    (Utilities|FlowControl|Delay 0.3)
    (Rendering|SetVisibility (Variables|/Script/Immortal_YiSunSin.WidgetStart|Getwidget _output_get) true false)
    (Variables|/Script/UMG.WidgetInteractionComponent|SetbShowDebug (Variables|Default|GetWidget%20Interaction%20L) true)
    (Variables|/Script/UMG.WidgetInteractionComponent|SetbShowDebug (Variables|Default|GetWidget%20Interaction%20R) true)
    (Variables|/Script/Immortal_YiSunSin.YiSunSinInstance|Setpos _yi_sun_sin_instance "90.000000,-200.000000,105.000000")
    (Variables|/Script/Immortal_YiSunSin.YiSunSinInstance|Setrot _yi_sun_sin_instance (Pawn|GetControlRotation (Game|GetPlayerController 0) :!class /Script/Engine.Controller))))

(event OnComponentEndOverlap(Box)
  (params (OverlappedComponent :type Primitive%20Component%20Object%20Reference) (OtherActor :type Actor%20Object%20Reference) (OtherComp :type Primitive%20Component%20Object%20Reference) (OtherBodyIndex :type Integer))
  (bind _widgetactor (Variables|Default|GetWidgetActor))
  (bind _audio (Variables|/Script/Immortal_YiSunSin.WidgetStart|Getaudio _widgetactor))
  (if (Utilities|String|Contains (Utilities|GetObjectName OtherComp) "Head")
    (Utilities|IsValid _audio
      (:Is%20Valid
        (Audio|Components|Audio|Stop _audio)
        (Actor|DestroyActor (Variables|Default|GetWidgetActor))
        (Variables|/Script/UMG.WidgetInteractionComponent|SetbShowDebug (Variables|Default|GetWidget%20Interaction%20L) false)
        (Variables|/Script/UMG.WidgetInteractionComponent|SetbShowDebug (Variables|Default|GetWidget%20Interaction%20R) false))
      (:Is%20Not%20Valid
        (Actor|DestroyActor (Variables|Default|GetWidgetActor))
        (Variables|/Script/UMG.WidgetInteractionComponent|SetbShowDebug (Variables|Default|GetWidget%20Interaction%20L) false)
        (Variables|/Script/UMG.WidgetInteractionComponent|SetbShowDebug (Variables|Default|GetWidget%20Interaction%20R) false)))))

(event EventBeginPlay
  (bind _returnvalue (Actor|GetActorOfClass "/Game/GN_Blueprint/Main/BP_mainPlayer.BP_mainPlayer_C"))
  (Variables|Default|SetPlayer _returnvalue)
  (Variables|Default|SetWidget%20Interaction%20L (Variables|/Script/Immortal_YiSunSin.mainPlayer|GetwidgetInteractionL _returnvalue))
  (Variables|Default|SetWidget%20Interaction%20R (Variables|/Script/Immortal_YiSunSin.mainPlayer|GetwidgetInteractionR _returnvalue))
  (bind _asyi_sun_sin_instance (Utilities|Casting|CastToYiSunSinInstance (Game|GetGameInstance)))
  (Variables|Default|SetYi%20Sun%20Sin%20Instance _asyi_sun_sin_instance))

(fn ConstructionScript)