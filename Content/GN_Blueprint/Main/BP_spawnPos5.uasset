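; BP_spawnPos5 is an overlap-triggered actor that reveals a widget for the main player to point at.
; On BeginPlay it waits briefly, then caches the BP_mainPlayer actor.
; Any actor overlap shows Widget61 and turns on ShowDebug for the player's left and right widget interaction components, without filtering the overlapping actor or validating the cached reference.
; Nothing hides the widget or the debug display again.
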(event EventBeginPlay
  (Utilities|FlowControl|Delay 1.0)
  (bind _returnvalue (Actor|GetActorOfClass "/Game/GN_Blueprint/Main/BP_mainPlayer.BP_mainPlayer_C")))

(event Collision|EventActorBeginOverlap
  (params (OtherActor :type Actor%20Object%20Reference))
  (Rendering|SetVisibility (Variables|Default|GetWidget6-1) true false)
  (bind _output_get (Variables|Default|SetWidget%20Interaction%20L (Variables|/Game/GN_Blueprint/Main/BP_mainPlayer.BP_mainPlayer_C|GetWidgetInteractionL (stale EventBeginPlay _returnvalue))))
  (bind _output_get_2 (Variables|Default|SetWidget%20Interaction%20R (Variables|/Game/GN_Blueprint/Main/BP_mainPlayer.BP_mainPlayer_C|GetWidgetInteractionR (stale EventBeginPlay _returnvalue))))
  (Variables|/Script/UMG.WidgetInteractionComponent|SetbShowDebug _output_get true)
  (Variables|/Script/UMG.WidgetInteractionComponent|SetbShowDebug _output_get_2 true))

(fn ConstructionScript)