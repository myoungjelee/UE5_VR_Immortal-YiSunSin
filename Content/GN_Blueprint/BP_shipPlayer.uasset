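; BP_shipPlayer is a ship player Blueprint that runs a level countdown and opens a level when time runs out.
; BeginPlay adds the BP_UI_timer widget to the viewport.
; Tick passes through a one-second Delay, which throttles it to step Seconds down and roll over Minutes about once per second.
; When both reach zero it calls OpenLevelByObjectReference; the overlap event and construction script are empty.
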(event EventBeginPlay
  ;[1 1 1] timer widget 띄우기
  (bind _returnvalue (UserInterface|CreateWidget "/Game/GN_Blueprint/BP_UI_timer.BP_UI_timer_C"))
  (UserInterface|Viewport|AddtoViewport _returnvalue 0))

(event Collision|EventActorBeginOverlap
  (params (OtherActor :type Actor%20Object%20Reference)))

(event EventTick
  (params (DeltaSeconds :type Float%20%28single-precision%29))
  (Utilities|FlowControl|Delay 1.0)
  (if (== (Variables|Default|GetSeconds) 0)
    (if (== (Variables|Default|GetMinutes) 0)
      ;[1 1 1] countDown 마치고 level open 하기
      (Game|OpenLevel(byObjectReference))
      (else
        (Variables|Default|SetSeconds 59)
        (Variables|Default|SetMinutes (- (Variables|Default|GetMinutes) 1))))
    (else
      (Variables|Default|SetSeconds (- (Variables|Default|GetSeconds) 1)))))

(fn ConstructionScript)