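; BP_ArcherPlayer is the player Blueprint for an archery game, managing its intro and end states.
; BeginPlay caches the timer widget and movie player, hides timer, score and bow, then after a short delay pauses and shows a game info UI.
; Tick polls the timer and score: zero time shows game over, while a score of one hides the HUD.
; All pauses use zero global time dilation.
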(event EventBeginPlay
  (bind _asbp_archer_timer (Utilities|Casting|CastToBP_ArcherTimer (UserInterface|GetUserWidgetObject (Variables|Default|GettimerUI))))
  (Variables|Default|Settimer _asbp_archer_timer)
  (bind _returnvalue (Actor|GetActorOfClass "/Game/SC/Blueprints/BP_ArcherMoviePlayer.BP_ArcherMoviePlayer_C"))
  (Variables|Default|SetMovie _returnvalue)
  (Rendering|SetVisibility (Variables|Default|GettimerUI) false false)
  (Rendering|SetVisibility (Variables|Default|GetscoreUI) false false)
  (Rendering|SetVisibility (Variables|Default|GetbowComp) false false)
  (Utilities|FlowControl|Delay 1.5)
  (Utilities|Time|SetGlobalTimeDilation 0.0)
  (Rendering|SetVisibility (Variables|Default|GetGameInfoUI1) true false))

(event Collision|EventActorBeginOverlap
  (params (OtherActor :type Actor%20Object%20Reference)))

(event EventTick
  (params (DeltaSeconds :type Float%20%28single-precision%29))
  (if (and (== (Variables|/Game/SC/UI/BP_ArcherTimer.BP_ArcherTimer_C|GetSeconds (Variables|Default|Gettimer)) 0) (== (Variables|/Game/SC/UI/BP_ArcherTimer.BP_ArcherTimer_C|GetMinutes (Variables|Default|Gettimer)) 0))
    (Utilities|Time|SetGlobalTimeDilation 0.0)
    (Rendering|SetVisibility (Variables|Default|GetgameoverUI) true false)
    (elif (== (Variables|/Script/Immortal_YiSunSin.ScoreUI|Getscore (Variables|Default|Getscore)) 1)
      (Utilities|Time|SetGlobalTimeDilation 0.0)
      (Rendering|SetVisibility (Variables|Default|GetscoreUI) false false)
      (Rendering|SetVisibility (Variables|Default|GettimerUI) false false))))

(fn ConstructionScript)