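; BP_WarriorPlayer is the warrior player Blueprint, which handles the return to the main level once the result UI appears.
; Tick polls the UI's visibility and uses a DoOnce, reset while the UI is hidden, to run the sequence a single time.
; After a short delay it fades the camera to black, then opens MainLevel.
; A BP_Trigger lookup is present but never runs.
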(event EventBeginPlay)

(event Collision|EventActorBeginOverlap
  (params (OtherActor :type Actor%20Object%20Reference)))

(event EventTick
  (params (DeltaSeconds :type Float%20%28single-precision%29))
  (if (Rendering|IsVisible (Variables|Default|GetresultUI))
    (Utilities|FlowControl|DoOnce false :!label _label
      (:Completed
        (Utilities|FlowControl|Delay 2.0)
        (CameraFades|StartCameraFade (Variables|/Script/Engine.PlayerController|GetPlayerCameraManager (Game|GetPlayerController 0)) 0.0 1.0 1.0 (Class|KismetMathLibrary|LinearColorBlack) false false)
        (Utilities|FlowControl|Delay 1.0)
        (Game|OpenLevel(byObjectReference) "/Game/Levels/MainLevel.MainLevel")))
    (else
      (goto _label Reset))))

(fn ConstructionScript)